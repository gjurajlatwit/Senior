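; Top-down player character that moves through Enhanced Input, messages overlapping NPCs on interact, and supports voice conversation with an AI persona, Tony.
; Holding T captures microphone audio and streams it into a runtime speech recognizer.
; Each recognized segment joins a history array, which VaRest posts to OpenAI chat completions with a hardcoded persona prompt.
; Replies appear briefly in a dialogue widget but are not added to the history.
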(event Custom|Text%20Prompt
  (params (Input%20Prompt :type String))
  ;[1 1 1] GPT Response
  (Development|PrintString "Promt ChatGPT" true true "(R=0.128853,G=1.000000,B=0.290327,A=1.000000)")
  (Variables|Default|SetInput%20Prompt (Utilities|String|JoinStringArray (Variables|Default|GetConvers_Array) " "))
  (bind _returnvalue (Class|VaRestSubsystem|ConstructVaRestRequestExt (|VaRestSubsystem) "POST" "json"))
  (Class|VaRestRequestJSON|SetRequestObject _returnvalue (|MakeJson "gpt-3.5-turbo" (Utilities|Array|MakeArray (|MakeJson "system" "You are Tony, Andy's lost brother. You are plotting a coup to overthrow the dominion. So you reach out to your brother who you haven't seen in a long time, because he thought you were killed. You talk in very short and concise sentences.") (|MakeJson "user" (Variables|Default|GetInput%20Prompt))) 1e+02))
  (Class|VaRestRequestJSON|SetHeader _returnvalue "Authorization" (Utilities|String|Append "Bearer " (Variables|Default|GetOpenAIKey)))
  (Class|VaRestRequestJSON|SetHeader _returnvalue "Content-Type" "application/json")
  (Class|VaRestRequestJSON|ProcessURL _returnvalue "https://api.openai.com/v1/chat/completions")
  (EventDispatchers|BindEventtoOnRequestComplete _returnvalue (delegate Custom|GPTRequestComplete))
  (EventDispatchers|BindEventtoOnRequestFail _returnvalue (delegate Custom|GPT%20REQUEST%20FAILED)))

(event Custom|GPTRequestComplete
  (params (Request :type Va%20Rest%20Request%20JSON%20Object%20Reference))
  ;[1 1 1] GPT Response
  (bind _returnvalue (Class|VaRestRequestJSON|GetResponseContentasString Request true))
  (if (Utilities|String|Contains _returnvalue "ERROR")
    (Development|PrintString _returnvalue true true "(R=1.000000,G=0.000000,B=0.082504,A=1.000000)" 1e+01)
    (else
      (bind _returnvalue_2 (UserInterface|CreateWidget "/Game/NPC/Dialogue_Text.Dialogue_Text_C" (Game|GetPlayerController 0)))
      (bind _output_get (Variables|Default|SetGUI _returnvalue_2))
      (UserInterface|Viewport|AddtoViewport _output_get 0)
      (Rendering|Components|TextRender|SetText (Variables|/Game/NPC/Dialogue_Text.Dialogue_Text_C|GetTextBlock_0 (Variables|Default|GetGUI)) (Utilities|Text|ToText(String) (|BreakJson (|BreakJson (Utilities|Array|Get(acopy) (Class|VaRestJsonObject|GetObjectArrayField (Class|VaRestRequestJSON|GetResponseObject Request) "choices"))))))
      (Utilities|FlowControl|Delay 5.0)
      (Viewport|RemoveAllWidgets))))

(event Custom|OnStartSpeechRecognition_Event
  (params (bSucceeded :type Boolean))
  (bind _returnvalue (Class|CapturableSoundWave|CreateCapturableSoundWave))
  (bind _output_get (Variables|Default|SetCapturableSoundWave _returnvalue))
  (EventDispatchers|BindEventtoOnPopulateAudioData _output_get (delegate Custom|OnPopulateAudioData_Event))
  (Class|CapturableSoundWave|StartCapture (Variables|Default|GetCapturableSoundWave)))

(event Custom|GPT%20REQUEST%20FAILED
  (params (Request :type Va%20Rest%20Request%20JSON%20Object%20Reference))
  ;[1 1 1] GPT Response
  (Development|PrintString "GPT REQUEST FAILED" true true "(R=1.000000,G=0.014152,B=0.123819,A=1.000000)"))

(event Custom|OnRecognitionFinished_Event
  (if (not (Class|CapturableSoundWave|IsCapturing (Variables|Default|GetCapturableSoundWave)))
    (Class|SpeechRecognizer|StopSpeechRecognition (Variables|Default|GetSpeechRecognizer))
    (Variables|Default|SetSpeechRecognizer 0)))

(event Custom|OnRecognitionError_Event
  (params (ShortErrorMessage :type String) (LongErrorMessage :type String))
  (Development|PrintString LongErrorMessage true true "(R=1.000000,G=0.000000,B=0.000000,A=1.000000)" 15.0))

(event Custom|OnRecognizedTextSegment_Event
  (params (RecognizedWords :type String))
  (Development|PrintString RecognizedWords true true "(R=1.000000,G=0.141020,B=0.869809,A=1.000000)" 12.0)
  (Utilities|Array|Add (Variables|Default|GetConvers_Array) (Utilities|String|Append "user:" RecognizedWords))
  (CallFunction|TextPrompt))

(event Custom|OnPopulateAudioData_Event
  (params (PopulatedAudioData :type Array%20of%20Floats%20%28single-precision%29))
  (bind _capturablesoundwave (Variables|Default|GetCapturableSoundWave))
  (Class|SpeechRecognizer|ProcessAudioData (Variables|Default|GetSpeechRecognizer) PopulatedAudioData (Math|Conversions|ToFloat(Integer) (Class|ImportedSoundWave|GetSampleRate _capturablesoundwave)) (Class|ImportedSoundWave|GetNumOfChannels _capturablesoundwave) false))

(event Input|EnhancedActionEvents|EnhancedInputActionIA_MOVE
  (params (ActionValue :type Vector%202D%20Structure) (ElapsedSeconds :type Float%20%28double-precision%29) (TriggeredSeconds :type Float%20%28double-precision%29) (InputAction :type Input%20Action%20Object%20Reference :default "/Game/INPUT/IA_MOVE.IA_MOVE"))
  (:Triggered
    (Pawn|Input|AddMovementInput "1.000000,0.000000,0.000000" (.x ActionValue) false)
    (Pawn|Input|AddMovementInput "0.000000,-1.000000,0.000000" (.y ActionValue) false)
    (Variables|Default|SetDirectionality (Math|Vector2D|MakeVector2D (.x ActionValue) (.y ActionValue))))
  (:Started
    (Variables|Default|SetIsHoldingMove true))
  (:Completed
    (Variables|Default|SetIsHoldingMove false)))

(event Input|EnhancedActionEvents|EnhancedInputActionIA_INTERACT
  (params (ActionValue :type Boolean) (ElapsedSeconds :type Float%20%28double-precision%29) (TriggeredSeconds :type Float%20%28double-precision%29) (InputAction :type Input%20Action%20Object%20Reference :default "/Game/NPC/IA_INTERACT.IA_INTERACT"))
  (:Started
    (for _array_element (Collision|GetOverlappingActors "/Game/NPC/TEST_NPC.TEST_NPC_C" :!class /Script/Engine.Actor)
      (if true
        (Class|NPCDIALOGUE|Interact(Message) _array_element)))))

(event Input|EnhancedActionEvents|EnhancedInputActionIA_INTERACT
  (params (ActionValue :type Boolean) (ElapsedSeconds :type Float%20%28double-precision%29) (TriggeredSeconds :type Float%20%28double-precision%29) (InputAction :type Input%20Action%20Object%20Reference :default "/Game/NPC/IA_INTERACT.IA_INTERACT"))
  (:Started
    (for _array_element (Collision|GetOverlappingActors "/Game/NPC/OfficeWorker1.OfficeWorker1_C" :!class /Script/Engine.Actor)
      (if true
        (Class|NPCDIALOGUE|Interact(Message) _array_element)))))

(event Input|EnhancedActionEvents|EnhancedInputActionIA_INTERACT
  (params (ActionValue :type Boolean) (ElapsedSeconds :type Float%20%28double-precision%29) (TriggeredSeconds :type Float%20%28double-precision%29) (InputAction :type Input%20Action%20Object%20Reference :default "/Game/NPC/IA_INTERACT.IA_INTERACT"))
  (:Started
    (for _array_element (Collision|GetOverlappingActors "/Game/NPC/OWF1.OWF1_C" :!class /Script/Engine.Actor)
      (if true
        (Class|NPCDIALOGUE|Interact(Message) _array_element)))))

(event EventBeginPlay
  (bind _asplayer_controller (Utilities|Casting|CastToPlayerController (Pawn|GetController)))
  (Input|AddMappingContext (PlayerController|LocalPlayerSubsystems|GetEnhancedInputLocalPlayerSubsystem _asplayer_controller) "/Game/INPUT/IMC_TOPDOWN.IMC_TOPDOWN" 0 "(bIgnoreAllPressedKeysUntilRelease=True,bForceImmediately=False)"))

(event Input|KeyboardEvents|T
  (params (Key :type Key%20Structure :default "None"))
  (:Pressed
    (bind _returnvalue (Class|SpeechRecognizer|CreateSpeechRecognizer))
    (bind _output_get (Variables|Default|SetSpeechRecognizer _returnvalue))
    (EventDispatchers|BindEventtoOnRecognitionFinished _output_get (delegate Custom|OnRecognitionFinished_Event))
    (EventDispatchers|BindEventtoOnRecognitionError (Variables|Default|GetSpeechRecognizer) (delegate Custom|OnRecognitionError_Event))
    (EventDispatchers|BindEventtoOnRecognizedTextSegment (Variables|Default|GetSpeechRecognizer) (delegate Custom|OnRecognizedTextSegment_Event))
    (Class|SpeechRecognizer|SetStreamingDefaults (Variables|Default|GetSpeechRecognizer))
    (Class|SpeechRecognizer|SetLanguage (Variables|Default|GetSpeechRecognizer) "En")
    (Class|SpeechRecognizer|StartSpeechRecognition (Variables|Default|GetSpeechRecognizer) (delegate Custom|OnStartSpeechRecognition_Event)))
  (:Released
    (Class|CapturableSoundWave|StopCapture (Variables|Default|GetCapturableSoundWave))
    (Class|SpeechRecognizer|ForceProcessPendingAudioData (Variables|Default|GetSpeechRecognizer))))

(fn ConstructionScript)